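; Enemy pursuer pawn that damages a living player, with an effect and sound, on capsule overlap or reaching them in a chase.
; Tick sets Roam or Chase Player by player distance.
; Self-recalling Roam and ChasePlayer events switch on that state and drive AIMoveTo, but nothing in this graph starts them.
; PawnSensing separately sets the HasSeenPlayer Blackboard key on sighting the player.
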(event OnSeePawn(PawnSensing)
  (params (Pawn :type Pawn%20Object%20Reference))
  (bind _asbp_learning_kit_player_character (Utilities|Casting|CastToBP_LearningKit_PlayerCharacter Pawn))
  (AI|Components|Blackboard|SetValueasBool (AI|GetBlackboard (AI|GetAIController self)) (Utilities|Name|MakeLiteralName "HasSeenPlayer") true)
  (if (Variables|/Game/LearningKit_Games/Blueprints/PlayerCharacter/BP_LearningKit_PlayerCharacter.BP_LearningKit_PlayerCharacter_C|GetIsDead _asbp_learning_kit_player_character)
    _))

(event OnComponentBeginOverlap(Capsule)
  (params (OverlappedComponent :type Primitive%20Component%20Object%20Reference) (OtherActor :type Actor%20Object%20Reference) (OtherComp :type Primitive%20Component%20Object%20Reference) (OtherBodyIndex :type Integer) (bFromSweep :type Boolean) (SweepResult :type Hit%20Result%20Structure%20%28by%20ref%29))
  (bind _returnvalue (Transformation|GetActorLocation))
  (bind _asbp_learning_kit_player_character (Utilities|Casting|CastToBP_LearningKit_PlayerCharacter OtherActor))
  (if (not (Variables|/Game/LearningKit_Games/Blueprints/PlayerCharacter/BP_LearningKit_PlayerCharacter.BP_LearningKit_PlayerCharacter_C|GetIsDead _asbp_learning_kit_player_character))
    (Game|Damage|ApplyDamage _asbp_learning_kit_player_character 5.0 0 0)
    (Effects|SpawnEmitteratLocation "/Game/LearningKit_Games/Assets/VFX/LightRay/vfx_lightray_card_01_P1_soft1_sea.vfx_lightray_card_01_P1_soft1_sea" _returnvalue)
    (Audio|PlaySoundatLocation "/Game/LearningKit_Robots/Audio/Bump_Metal_v3_Cue.Bump_Metal_v3_Cue" _returnvalue "0, 0, 0" 1.0 1.0 0.0 0 0 0 0)))

(event Custom|Roam
  (switch Utilities|FlowControl|Switch|SwitchonEAIState (Variables|Default|GetAIState)
    (:NewEnumerator1
      (AI|AIMoveTo self (.RandomLocation (AI|Navigation|GetRandomReachablePointinRadius (Transformation|GetActorLocation) 1e+03 0 0)) 0 5.0 false
        (:OnSuccess
          (Utilities|FlowControl|Delay 0.5)
          (CallFunction|Roam))))
    (:NewEnumerator2
      (CallFunction|ChasePlayer))))

(event Custom|Chase%20Player
  (bind _returnvalue (Game|GetPlayerCharacter 0))
  (bind _self self)
  (bind _returnvalue_2 (Transformation|GetActorLocation _self))
  (switch Utilities|FlowControl|Switch|SwitchonEAIState (Variables|Default|GetAIState)
    (:NewEnumerator1
      (CallFunction|Roam))
    (:NewEnumerator2
      (AI|AIMoveTo self "0, 0, 0" (Game|GetPlayerCharacter 0) 5.0 false
        (:OnSuccess
          (bind _asbp_learning_kit_player_character (Utilities|Casting|CastToBP_LearningKit_PlayerCharacter _returnvalue))
          (if (Variables|/Game/LearningKit_Games/Blueprints/PlayerCharacter/BP_LearningKit_PlayerCharacter.BP_LearningKit_PlayerCharacter_C|GetIsDead _asbp_learning_kit_player_character)
            _
            (else
              (Game|Damage|ApplyDamage _returnvalue 5.0 0 0)
              (Effects|SpawnEmitteratLocation "/Game/LearningKit_Games/Assets/VFX/LightRay/vfx_lightray_card_01_P1_soft1_sea.vfx_lightray_card_01_P1_soft1_sea" _returnvalue_2)
              (Audio|PlaySoundatLocation "/Game/LearningKit_Robots/Audio/Bump_Metal_v3_Cue.Bump_Metal_v3_Cue" _returnvalue_2 "0, 0, 0" 1.0 1.0 0.0 0 0 0 0)))
          (Utilities|FlowControl|Delay 1.0)
          (CallFunction|ChasePlayer))
        (:OnFail
          (CallFunction|Roam))))))

(event EventBeginPlay)

(event Collision|EventActorBeginOverlap
  (params (OtherActor :type Actor%20Object%20Reference)))

(event EventTick
  (params (DeltaSeconds :type Float%20%28single-precision%29))
  (if (< (Math|Vector|Distance(Vector) (Transformation|GetActorLocation) (Transformation|GetActorLocation (Game|GetPlayerCharacter 0))) 6e+02)
    (Variables|Default|SetAIState "NewEnumerator2")
    (else
      (Variables|Default|SetAIState "NewEnumerator1"))))

(fn ConstructionScript)